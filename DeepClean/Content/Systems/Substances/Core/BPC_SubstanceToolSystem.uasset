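; Substance tool component that sprays stored sand onto surfaces as runtime patch actors and deducts the amount deposited.
; TrySpraySand traces for an upward-facing surface, or steps downhill from too-steep hits to find a rest spot.
; Five samples around that point are resolved and grouped by hit actor and component.
; Coplanar sets form one pile; others split the amount by weight, merging into nearby matching patches or spawning new ones.
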(fn `BuildSubstanceDepositGroups`
  (params (ResolvedSampleHits :type "Array of HitResult Structure"))
  (returns (DepositGroups :type "Array of /Game/Systems/Substances/Core/ST_SubstanceDepositGroup Structure"))
  (locals (WorkingGroups :type "Array of /Game/Systems/Substances/Core/ST_SubstanceDepositGroup Structure") (CurrentHit :type "HitResult Structure") (MatchedGroupIndex :type Integer) (UpdatedMemberHits :type "Array of HitResult Structure"))
  (bind _updatedmemberhits (`local.UpdatedMemberHits`))
  (bind _currenthit (`local.CurrentHit`))
  (bind _currenthit_2 (`local.CurrentHit`))
  (bind (_bblockinghit _binitialoverlap _time _distance _location _impactpoint _normal _impactnormal _physmat _hitactor _hitcomponent) (`GameplayStatics.BreakHitResult` (`local.CurrentHit`)))
  (bind (_bblockinghit_2 _binitialoverlap_2 _time_2 _distance_2 _location_2 _impactpoint_2 _normal_2 _impactnormal_2) (`GameplayStatics.BreakHitResult` _currenthit))
  (bind (_bblockinghit_3 _binitialoverlap_3 _time_3 _distance_3 _location_3 _impactpoint_3 _normal_3 _impactnormal_3) (`GameplayStatics.BreakHitResult` _currenthit_2))
  (bind (_representativehit _weightedlocationsum _weightednormalsum _totalweight _samplecount _memberhits) (break `/Game/Systems/Substances/Core/ST_SubstanceDepositGroup` (`|GetArrayItem` (`local.WorkingGroups`) (`local.MatchedGroupIndex`))))
  (`KismetArrayLibrary.Array_Clear` (`local.WorkingGroups`))
  (for _array_element ResolvedSampleHits
    (set `local.CurrentHit` _array_element)
    (set `local.MatchedGroupIndex` -1)
    (for (_array_element_2 _array_index) (`local.WorkingGroups`)
      (bind (_bblockinghit_4 _binitialoverlap_4 _time_4 _distance_4 _location_4 _impactpoint_4 _normal_4 _impactnormal_4 _physmat_2 _hitactor_2 _hitcomponent_2) (`GameplayStatics.BreakHitResult` (`.RepresentativeHit_2_FABFFE334ABA5EA1B8658A98024AF317` (break `/Game/Systems/Substances/Core/ST_SubstanceDepositGroup` _array_element_2))))
      (if (and (== _hitactor _hitactor_2) (== _hitcomponent _hitcomponent_2))
        (set `local.MatchedGroupIndex` _array_index)
        (break)))
    (if (>= (`local.MatchedGroupIndex`) 0)
      (set `local.UpdatedMemberHits` _memberhits)
      (`KismetArrayLibrary.Array_Add` _updatedmemberhits _currenthit_2)
      (`KismetArrayLibrary.Array_Set` (`local.WorkingGroups`) (`local.MatchedGroupIndex`) (make `/Game/Systems/Substances/Core/ST_SubstanceDepositGroup` _representativehit (+ _weightedlocationsum _impactpoint_3) (+ _weightednormalsum _impactnormal_3) (+ _totalweight 1.0) (+ _samplecount 1) _updatedmemberhits))
      (else
        (`KismetArrayLibrary.Array_Add` (`local.WorkingGroups`) (make `/Game/Systems/Substances/Core/ST_SubstanceDepositGroup` _currenthit _impactpoint_2 _impactnormal_2 1.0 1 (`|MakeArray` _currenthit))))))
  (return (`local.WorkingGroups`)))

(fn `CleanupRuntimeSubstancePatches`
  (bind (_arrayindex _arrayelement) (`/Engine/EditorBlueprintResources/StandardMacros.ReverseForEachLoop` (`self.RuntimeSubstancePatches`))
    (:`LoopBody`
      (`/Engine/EditorBlueprintResources/StandardMacros.IsValid` _arrayelement
        (:`Is Not Valid`
          (`KismetArrayLibrary.Array_Remove` (`self.RuntimeSubstancePatches`) _arrayindex))))))

(fn `CollectResolvedDepositSamples`
  (params (CenterHitResult :type "HitResult Structure") (SampleRadius :type "Float (double-precision)"))
  (returns (ResolvedSampleHits :type "Array of HitResult Structure"))
  (locals (CollectedHits :type "Array of HitResult Structure"))
  (bind (_bblockinghit _binitialoverlap _time _distance _location _impactpoint _normal _impactnormal) (`GameplayStatics.BreakHitResult` CenterHitResult))
  (bind _returnvalue (`KismetMathLibrary.FMax` SampleRadius))
  (bind _returnvalue_2 (`KismetMathLibrary.MakeRotFromZ` _impactnormal))
  (bind _returnvalue_3 (* (`KismetMathLibrary.GetForwardVector` _returnvalue_2) _returnvalue))
  (bind _returnvalue_4 (* (`KismetMathLibrary.GetRightVector` _returnvalue_2) _returnvalue))
  (`KismetArrayLibrary.Array_Clear` (`local.CollectedHits`))
  (for _array_element (`|MakeArray` _impactpoint (+ _impactpoint _returnvalue_3) (- _impactpoint _returnvalue_3) (+ _impactpoint _returnvalue_4) (- _impactpoint _returnvalue_4))
    (bind (_sampleresolved _samplehitresult) (`self.ResolveDepositSample` _array_element))
    (if _sampleresolved
      (`KismetArrayLibrary.Array_Add` (`local.CollectedHits`) _samplehitresult)))
  (return (`local.CollectedHits`)))

(fn `CommitSubstanceDepositGroups`
  (params (DepositGroups :type "Array of /Game/Systems/Substances/Core/ST_SubstanceDepositGroup Structure") (RuntimePatchClass :type "/Game/Systems/Substances/Core/BP_SubstancePatchBase Class Reference") (RequiredSubstanceType :type "/Game/Systems/Substances/Core/E_SubstanceType Enum" :default "NewEnumerator0") (TotalAmountToDeposit :type "Float (double-precision)"))
  (returns (CommittedAmount :type "Float (double-precision)") (AnyDeposited :type Boolean))
  (locals (SafeTotalAmount :type "Float (double-precision)") (TotalGroupWeight :type "Float (double-precision)") (RunningCommittedAmount :type "Float (double-precision)") (GroupLocation :type "Vector Structure") (GroupNormal :type "Vector Structure") (GroupAmount :type "Float (double-precision)") (AllMembersOnSamePlane :type Boolean))
  (bind _groupamount (`local.GroupAmount`))
  (bind _runningcommittedamount (`local.RunningCommittedAmount`))
  (bind (_bblockinghit _binitialoverlap _time _distance _location _impactpoint _normal _impactnormal _physmat _hitactor _hitcomponent) (`GameplayStatics.BreakHitResult` (`.RepresentativeHit_2_FABFFE334ABA5EA1B8658A98024AF317` (break `/Game/Systems/Substances/Core/ST_SubstanceDepositGroup` (`|GetArrayItem` DepositGroups)))))
  (set `local.SafeTotalAmount` (`KismetMathLibrary.FMax` TotalAmountToDeposit))
  (bind _usesinglepile (`self.ShouldUseSinglePile` DepositGroups))
  (if _usesinglepile
    (bind (_targetpatch _deposited) (`self.DepositSubstanceAmountAtSurface` RuntimePatchClass RequiredSubstanceType _impactpoint (`KismetMathLibrary.Normal` _impactnormal) _hitactor _hitcomponent (`local.SafeTotalAmount`)))
    (if _deposited
      (set `local.RunningCommittedAmount` (`local.SafeTotalAmount`))
      (return (`local.SafeTotalAmount`) true))
    (else
      (set `local.TotalGroupWeight` 0.0)
      (set `local.RunningCommittedAmount` 0.0)
      (if (and (and (> (`local.SafeTotalAmount`) 0.001) (> (`KismetArrayLibrary.Array_Length` DepositGroups) 0)) (`KismetSystemLibrary.IsValidClass` RuntimePatchClass))
        (for _array_element DepositGroups
          (bind (_representativehit _weightedlocationsum _weightednormalsum _totalweight) (break `/Game/Systems/Substances/Core/ST_SubstanceDepositGroup` _array_element))
          (if (> _totalweight 0.001)
            (set `local.TotalGroupWeight` (+ (`local.TotalGroupWeight`) _totalweight))))
        (if (> (`local.TotalGroupWeight`) 0.001)
          (for _array_element_2 DepositGroups
            (bind (_representativehit_2 _weightedlocationsum_2 _weightednormalsum_2 _totalweight_2 _samplecount _memberhits) (break `/Game/Systems/Substances/Core/ST_SubstanceDepositGroup` _array_element_2))
            (if (> _totalweight_2 0.001)
              (set `local.GroupLocation` (/ _weightedlocationsum_2 _totalweight_2))
              (bind (_bblockinghit_2 _binitialoverlap_2 _time_2 _distance_2 _location_2 _impactpoint_2 _normal_2 _impactnormal_2 _physmat_2 _hitactor_2 _hitcomponent_2) (`GameplayStatics.BreakHitResult` _representativehit_2))
              (bind _returnvalue (`KismetMathLibrary.Normal` _weightednormalsum_2))
              (set `local.GroupNormal` (`KismetMathLibrary.SelectVector` (`KismetMathLibrary.Normal` _impactnormal_2) _returnvalue (`KismetMathLibrary.Vector_IsNearlyZero` _returnvalue)))
              (set `local.GroupAmount` (* (`local.SafeTotalAmount`) (/ _totalweight_2 (`local.TotalGroupWeight`))))
              (bind _returnvalue_2 (`KismetArrayLibrary.Array_Length` _memberhits))
              (if (> _returnvalue_2 0)
                (for _array_element_3 _memberhits
                  (bind (_bblockinghit_3 _binitialoverlap_3 _time_3 _distance_3 _location_3 _impactpoint_3 _normal_3 _impactnormal_3 _physmat_3 _hitactor_3 _hitcomponent_3) (`GameplayStatics.BreakHitResult` _array_element_3))
                  (bind _returnvalue_3 (/ (`local.GroupAmount`) _returnvalue_2))
                  (bind (_targetpatch_2 _deposited_2) (`self.DepositSubstanceAmountAtSurface` RuntimePatchClass RequiredSubstanceType (`local.GroupLocation`) (`local.GroupNormal`) _hitactor_3 _hitcomponent_3 _returnvalue_3))
                  (if _deposited_2
                    (set `local.RunningCommittedAmount` (+ (`local.RunningCommittedAmount`) _returnvalue_3))))
                (else
                  (bind (_targetpatch_3 _deposited_3) (`self.DepositSubstanceAmountAtSurface` RuntimePatchClass RequiredSubstanceType (`local.GroupLocation`) (`local.GroupNormal`) _hitactor_2 _hitcomponent_2 _groupamount))
                  (if _deposited_3
                    (set `local.RunningCommittedAmount` (+ (`local.RunningCommittedAmount`) _groupamount)))))))
          (return (`KismetMathLibrary.FClamp` _runningcommittedamount 0.0 (`local.SafeTotalAmount`)) (> _runningcommittedamount 0.0))
          (else
            (return 0.0 false)))
        (else
          (return 0.0 false))))))

(fn `DepositSandAtSurface`
  (params (WorldLocation :type "Vector Structure") (SurfaceNormal :type "Vector Structure") (SurfaceOwner :type "Actor Object Reference") (SupportComponent :type "PrimitiveComponent Object Reference"))
  (bind (_foundpatch _found) (`self.FindNearbyRuntimeSubstancePatch` WorldLocation "NewEnumerator0" SurfaceOwner SupportComponent))
  (if _found
    (`/Game/Systems/Substances/Core/BP_SubstancePatchBase.AddRuntimeSubstanceCell` _foundpatch WorldLocation SurfaceNormal)
    (set `self.StoredSandAmount` (`KismetMathLibrary.FClamp` (- (`self.StoredSandAmount`) (`self.SandAmountPerCell`)) 0.0 (`self.MaxStoredSandAmount`)))
    (else
      (`self.SpawnRuntimeSandPatchAtSurface` WorldLocation SurfaceNormal SurfaceOwner SupportComponent))))

(fn `DepositSubstanceAmountAtSurface`
  (params (RuntimePatchClass :type "/Game/Systems/Substances/Core/BP_SubstancePatchBase Class Reference") (RequiredSubstanceType :type "/Game/Systems/Substances/Core/E_SubstanceType Enum" :default "NewEnumerator0") (WorldLocation :type "Vector Structure") (SurfaceNormal :type "Vector Structure") (SurfaceOwner :type "Actor Object Reference") (SupportComponent :type "PrimitiveComponent Object Reference") (AmountToDeposit :type "Float (double-precision)"))
  (returns (TargetPatch :type "/Game/Systems/Substances/Core/BP_SubstancePatchBase Object Reference") (Deposited :type Boolean))
  (locals (SafeAmount :type "Float (double-precision)"))
  (bind _safeamount (`local.SafeAmount`))
  (set `local.SafeAmount` (`KismetMathLibrary.FMax` AmountToDeposit))
  (if (and (> (`local.SafeAmount`) 0.001) (`KismetSystemLibrary.IsValidClass` RuntimePatchClass))
    (bind (_foundpatch _found) (`self.FindNearbyRuntimeSubstancePatch` WorldLocation RequiredSubstanceType SurfaceOwner SupportComponent))
    (if _found
      (`/Game/Systems/Substances/Core/BP_SubstancePatchBase.AddRuntimeSubstanceCellWithAmount` _foundpatch WorldLocation SurfaceNormal _safeamount)
      (return _foundpatch true)
      (else
        (bind (_spawnedpatch _spawnsucceeded) (`self.SpawnRuntimeSubstancePatchAtSurfaceWithAmount` RuntimePatchClass RequiredSubstanceType WorldLocation SurfaceNormal SurfaceOwner SupportComponent _safeamount))
        (return _spawnedpatch _spawnsucceeded)))
    (else
      (return null false))))

(fn `FindGravityFallbackSurface`
  (params (ImpactLocation :type "Vector Structure"))
  (returns (FallbackFound :type Boolean) (FallbackHitResult :type "HitResult Structure"))
  (`KismetSystemLibrary.LineTraceSingle` :`Start` (+ ImpactLocation (0.0 0.0 20.0)) :`End` (+ ImpactLocation (0.0 0.0 -300.0)) :`TraceChannel` "TraceTypeQuery1" :`DrawDebugType` "ForDuration")
  (return false))

(fn `FindGravityRestSurface`
  (params (InitialHitResult :type "HitResult Structure"))
  (returns (RestSurfaceFound :type Boolean) (RestHitResult :type "HitResult Structure"))
  (locals (DownhillDirection :type "Vector Structure") (CandidateFound :type Boolean) (CandidateHitResult :type "HitResult Structure"))
  (bind (_bblockinghit _binitialoverlap _time _distance _location _impactpoint _normal _impactnormal) (`GameplayStatics.BreakHitResult` InitialHitResult))
  (bind _gravitysearchmaxsteps (`self.GravitySearchMaxSteps`))
  (bind _gravitysearchstep (`self.GravitySearchStep`))
  (bind _gravityprobeheight (`self.GravityProbeHeight`))
  (bind _gravitysearchdistance (`self.GravitySearchDistance`))
  (`KismetSystemLibrary.PrintString` (`KismetTextLibrary.Conv_TextToString` (`|FormatText` "GRAVITY SEARCH START | Step={Step} | MaxSteps={MaxSteps} | Distance={Distance} | ProbeHeight={ProbeHeight}" _gravitysearchstep _gravitysearchmaxsteps _gravitysearchdistance _gravityprobeheight)))
  (set `local.CandidateFound` false)
  (set `local.DownhillDirection` (`KismetMathLibrary.Normal` (`KismetMathLibrary.MakeVector` (.x _impactnormal) (.y _impactnormal))))
  (for _index (range 1 (+ _gravitysearchmaxsteps 1))
    (bind _returnvalue (+ (+ _impactpoint (* (* (`KismetMathLibrary.Conv_IntToDouble` _index) _gravitysearchstep) (`local.DownhillDirection`))) (`KismetMathLibrary.MakeVector` 0.0 0.0 _gravityprobeheight)))
    (`KismetSystemLibrary.PrintString` (`KismetTextLibrary.Conv_TextToString` (`|FormatText` "GRAVITY LOOP STEP | Index={Index} | Start={SearchStart}" _index (`KismetStringLibrary.Conv_VectorToString` _returnvalue))))
    (bind (_hitfound _hitresult _surfaceaccepted) (`self.FindSpraySurface` _returnvalue (0.0 0.0 -1.0) _gravitysearchdistance))
    (if _surfaceaccepted
      (bind (_bblockinghit_2 _binitialoverlap_2 _time_2 _distance_2 _location_2 _impactpoint_2 _normal_2 _impactnormal_2 _physmat _hitactor _hitcomponent) (`GameplayStatics.BreakHitResult` _hitresult))
      (`KismetSystemLibrary.DrawDebugSphere` _impactpoint_2 20.0 12 (struct :`G` 1.0 :`A` 1.0) 5.0 2.0)
      (`KismetSystemLibrary.PrintString` (`KismetTextLibrary.Conv_TextToString` (`|FormatText` "REST SURFACE FOUND | ImpactPoint={ImpactPoint} | ImpactNormal={ImpactNormal} | HitActor={HitActor} | HitComponent={HitComponent}" (`KismetStringLibrary.Conv_VectorToString` _impactpoint_2) (`KismetStringLibrary.Conv_VectorToString` _impactnormal_2) (`KismetSystemLibrary.GetObjectName` _hitactor) (`KismetSystemLibrary.GetObjectName` _hitcomponent))))
      (set `local.CandidateHitResult` _hitresult)
      (set `local.CandidateFound` true)
      (break)))
  (return (`local.CandidateFound`) (`local.CandidateHitResult`)))

(fn `FindNearbyRuntimeSubstancePatch`
  (params (WorldLocation :type "Vector Structure") (RequiredSubstanceType :type "/Game/Systems/Substances/Core/E_SubstanceType Enum" :default "NewEnumerator0") (RequiredSurfaceOwner :type "Actor Object Reference") (RequiredSupportComponent :type "PrimitiveComponent Object Reference"))
  (returns (FoundPatch :type "/Game/Systems/Substances/Core/BP_SubstancePatchBase Object Reference") (Found :type Boolean))
  (locals (NearestPatch :type "/Game/Systems/Substances/Core/BP_SubstancePatchBase Object Reference") (NearestDistanceSquared :type "Float (double-precision)"))
  (bind _nearestpatch (`local.NearestPatch`))
  (`self.CleanupRuntimeSubstancePatches`)
  (set `local.NearestDistanceSquared` (* (`self.RuntimePatchMergeRadius`) (`self.RuntimePatchMergeRadius`)))
  (for _array_element (`self.RuntimeSubstancePatches`)
    (`/Engine/EditorBlueprintResources/StandardMacros.IsValid` _array_element
      (:`Is Valid`
        (if (and (`|EnumEquality` (`/Game/Systems/Substances/Core/BP_SubstancePatchBase.SubstanceType` _array_element) RequiredSubstanceType) (== (`/Game/Systems/Substances/Core/BP_SubstancePatchBase.SurfaceOwner` _array_element) RequiredSurfaceOwner) (== (`/Game/Systems/Substances/Core/BP_SubstancePatchBase.SupportComponent` _array_element) RequiredSupportComponent))
          (bind _returnvalue (`KismetMathLibrary.Vector_DistanceSquared` WorldLocation (`Actor.K2_GetActorLocation` _array_element)))
          (if (<= _returnvalue (`local.NearestDistanceSquared`))
            (set `local.NearestDistanceSquared` _returnvalue)
            (set `local.NearestPatch` _array_element))))))
  (`/Engine/EditorBlueprintResources/StandardMacros.IsValid` _nearestpatch
    (:`Is Valid`
      (return _nearestpatch true))
    (:`Is Not Valid`
      (return null false))))

(fn `FindSpraySurface`
  (params (StartLocation :type "Vector Structure") (ForwardDirection :type "Vector Structure") (TraceDistance :type "Float (double-precision)"))
  (returns (HitFound :type Boolean) (HitResult :type "HitResult Structure") (SurfaceAccepted :type Boolean))
  (bind (_outhit _returnvalue) (`KismetSystemLibrary.LineTraceSingle` StartLocation (+ StartLocation (* ForwardDirection TraceDistance)) "TraceTypeQuery1"))
  (return _returnvalue _outhit (and _returnvalue (>= (`KismetMathLibrary.Dot_VectorVector` (`.ImpactNormal` (`GameplayStatics.BreakHitResult` _outhit)) (`KismetMathLibrary.MakeVector` 0.0 0.0 1.0)) (`self.MinimumSurfaceUpDot`)))))

(fn `ResolveDepositSample`
  (params (SampleWorldLocation :type "Vector Structure"))
  (returns (SampleResolved :type Boolean) (SampleHitResult :type "HitResult Structure"))
  (bind (_hitfound _hitresult _surfaceaccepted) (`self.FindSpraySurface` (+ SampleWorldLocation (`KismetMathLibrary.MakeVector` 0.0 0.0 (`self.GravityProbeHeight`))) (`KismetMathLibrary.MakeVector` 0.0 0.0 -1.0) (`self.GravitySearchDistance`)))
  (if _surfaceaccepted
    (return true _hitresult)
    (elif _hitfound
      (bind (_restsurfacefound _resthitresult) (`self.FindGravityRestSurface` _hitresult))
      (if _restsurfacefound
        (return true _resthitresult)
        (else
          (return false)))
      (else
        (return false)))))

(fn `ShouldUseSinglePile`
  (params (DepositGroups :type "Array of /Game/Systems/Substances/Core/ST_SubstanceDepositGroup Structure") (ExpectedSampleCount :type Integer :default 5) (PlaneTolerance :type "Float (double-precision)" :default 5.0))
  (returns (UseSinglePile :type Boolean))
  (locals (AllMembersOnSamePlane :type Boolean))
  (bind _returnvalue (`KismetArrayLibrary.Array_Length` DepositGroups))
  (bind (_representativehit _weightedlocationsum _weightednormalsum _totalweight _samplecount _memberhits) (break `/Game/Systems/Substances/Core/ST_SubstanceDepositGroup` (`|GetArrayItem` DepositGroups)))
  (bind _returnvalue_2 (`KismetArrayLibrary.Array_Length` _memberhits))
  (bind (_bblockinghit _binitialoverlap _time _distance _location _impactpoint _normal _impactnormal) (`GameplayStatics.BreakHitResult` _representativehit))
  (`KismetSystemLibrary.PrintString` (`KismetStringLibrary.Concat_StrStr` "GroupCount = " (`KismetStringLibrary.Conv_IntToString` _returnvalue)) true true (struct :`G` 0.66 :`B` 1.0 :`A` 1.0) 5.0)
  (if (== _returnvalue 1)
    (`KismetSystemLibrary.PrintString` (`KismetStringLibrary.Concat_StrStr` "MemberHitCount = " (`KismetStringLibrary.Conv_IntToString` _returnvalue_2)) true true (struct :`G` 0.66 :`B` 1.0 :`A` 1.0) 5.0)
    (if (== _returnvalue_2 ExpectedSampleCount)
      (set `local.AllMembersOnSamePlane` true)
      (for _array_element _memberhits
        (bind _returnvalue_3 (`KismetMathLibrary.Abs` (`KismetMathLibrary.Dot_VectorVector` (- (`.ImpactPoint` (`GameplayStatics.BreakHitResult` _array_element)) _impactpoint) (`KismetMathLibrary.Normal` _impactnormal))))
        (`KismetSystemLibrary.PrintString` (`KismetStringLibrary.Concat_StrStr` "PlaneDistance = " (`KismetStringLibrary.Conv_DoubleToString` _returnvalue_3)) true true (struct :`G` 0.66 :`B` 1.0 :`A` 1.0) 5.0)
        (set `local.AllMembersOnSamePlane` (and (<= _returnvalue_3 PlaneTolerance) (`local.AllMembersOnSamePlane`))))
      (return (`local.AllMembersOnSamePlane`))
      (else
        (return false)))
    (else
      (return false))))

(fn `SpawnRuntimeSandPatchAtSurface`
  (params (WorldLocation :type "Vector Structure") (SurfaceNormal :type "Vector Structure") (SurfaceOwner :type "Actor Object Reference") (SupportComponent :type "PrimitiveComponent Object Reference"))
  (bind _returnvalue (`|SpawnActorFromClass` "/Game/Systems/Substances/Core/BP_RuntimeSandPatch.BP_RuntimeSandPatch_C" (`KismetMathLibrary.MakeTransform` (+ WorldLocation (* SurfaceNormal 2.0)) (`KismetMathLibrary.MakeRotFromZ` SurfaceNormal)) "AlwaysSpawn" "MultiplyWithRoot" null SurfaceOwner SupportComponent null))
  (`KismetArrayLibrary.Array_AddUnique` (`self.RuntimeSubstancePatches`) _returnvalue)
  (set `self.ActiveRuntimeSandPatch` _returnvalue)
  (set `self.StoredSandAmount` (`KismetMathLibrary.FClamp` (- (`self.StoredSandAmount`) (`self.SandAmountPerCell`)) 0.0 (`self.MaxStoredSandAmount`))))

(fn `SpawnRuntimeSubstancePatchAtSurfaceWithAmount`
  (params (RuntimePatchClass :type "/Game/Systems/Substances/Core/BP_SubstancePatchBase Class Reference") (RequiredSubstanceType :type "/Game/Systems/Substances/Core/E_SubstanceType Enum" :default "NewEnumerator0") (WorldLocation :type "Vector Structure") (SurfaceNormal :type "Vector Structure") (SurfaceOwner :type "Actor Object Reference") (SupportComponent :type "PrimitiveComponent Object Reference") (InitialAmount :type "Float (double-precision)"))
  (returns (SpawnedPatch :type "/Game/Systems/Substances/Core/BP_SubstancePatchBase Object Reference") (SpawnSucceeded :type Boolean))
  (locals (SafeAmount :type "Float (double-precision)"))
  (bind _returnvalue (`KismetMathLibrary.MakeRotFromZ` SurfaceNormal))
  (bind _safeamount (`local.SafeAmount`))
  (set `local.SafeAmount` (`KismetMathLibrary.FMax` InitialAmount))
  (if (and (> (`local.SafeAmount`) 0.001) (`KismetSystemLibrary.IsValidClass` RuntimePatchClass))
    (`KismetSystemLibrary.PrintString` (`KismetStringLibrary.Conv_VectorToString` SurfaceNormal))
    (`KismetSystemLibrary.PrintString` (`KismetStringLibrary.Conv_RotatorToString` _returnvalue))
    (bind _returnvalue_2 (`|SpawnActorFromClass` RuntimePatchClass (`KismetMathLibrary.MakeTransform` (+ WorldLocation (* SurfaceNormal 2.0)) _returnvalue) "AlwaysSpawn" "MultiplyWithRoot" null null null null))
    (`/Engine/EditorBlueprintResources/StandardMacros.IsValid` _returnvalue_2
      (:`Is Valid`
        (set `/Game/Systems/Substances/Core/BP_SubstancePatchBase.SubstanceType` RequiredSubstanceType _returnvalue_2)
        (set `/Game/Systems/Substances/Core/BP_SubstancePatchBase.SurfaceOwner` SurfaceOwner _returnvalue_2)
        (set `/Game/Systems/Substances/Core/BP_SubstancePatchBase.SupportComponent` SupportComponent _returnvalue_2)
        (set `/Game/Systems/Substances/Core/BP_SubstancePatchBase.MaxAmount` _safeamount _returnvalue_2)
        (set `/Game/Systems/Substances/Core/BP_SubstancePatchBase.StartingAmount` _safeamount _returnvalue_2)
        (set `/Game/Systems/Substances/Core/BP_SubstancePatchBase.CurrentAmount` _safeamount _returnvalue_2)
        (`/Game/Systems/Substances/Core/BP_SubstancePatchBase.ApplyLatestRuntimeCellVisualAmount` _returnvalue_2 _safeamount)
        (`KismetArrayLibrary.Array_AddUnique` (`self.RuntimeSubstancePatches`) _returnvalue_2)
        (return _returnvalue_2 true))
      (:`Is Not Valid`
        (return null false)))
    (else
      (return null false))))

(fn `TrySpraySand`
  (params (StartLocation :type "Vector Structure") (ForwardDirection :type "Vector Structure"))
  (if (>= (`self.StoredSandAmount`) (`self.SandAmountPerCell`))
    (bind (_hitfound _hitresult _surfaceaccepted) (`self.FindSpraySurface` StartLocation ForwardDirection (`self.SandSprayRange`)))
    (if _surfaceaccepted
      (bind _resolvedsamplehits (`self.CollectResolvedDepositSamples` _hitresult 75.0))
      (bind _depositgroups (`self.BuildSubstanceDepositGroups` _resolvedsamplehits))
      (bind (_committedamount _anydeposited) (`self.CommitSubstanceDepositGroups` _depositgroups "/Game/Systems/Substances/Core/BP_RuntimeSandPatch.BP_RuntimeSandPatch_C" "NewEnumerator0" (`self.SandAmountPerCell`)))
      (if _anydeposited
        (set `self.StoredSandAmount` (`KismetMathLibrary.FClamp` (- (`self.StoredSandAmount`) _committedamount) 0.0 (`self.MaxStoredSandAmount`))))
      (elif _hitfound
        (bind (_restsurfacefound _resthitresult) (`self.FindGravityRestSurface` _hitresult))
        (if _restsurfacefound
          (bind _resolvedsamplehits_2 (`self.CollectResolvedDepositSamples` _resthitresult 75.0))
          (bind _depositgroups_2 (`self.BuildSubstanceDepositGroups` _resolvedsamplehits_2))
          (bind (_committedamount_2 _anydeposited_2) (`self.CommitSubstanceDepositGroups` _depositgroups_2 "/Game/Systems/Substances/Core/BP_RuntimeSandPatch.BP_RuntimeSandPatch_C" "NewEnumerator0" (`self.SandAmountPerCell`)))
          (if _anydeposited_2
            (set `self.StoredSandAmount` (`KismetMathLibrary.FClamp` (- (`self.StoredSandAmount`) _committedamount_2) 0.0 (`self.MaxStoredSandAmount`)))))))))