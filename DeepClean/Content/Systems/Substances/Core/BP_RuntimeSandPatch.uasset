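; BP_RuntimeSandPatch is a sand substance patch that grows at runtime, one instanced clump at a time.
; Each added cell places a SandClumps instance just off the surface, aligned to its normal with random yaw, and updates cell count and amounts.
; The amount-specific variant adds a given quantity and shrinks the newest clump along a power curve for partial amounts.
; Depletion sets a very short lifespan without running the parent handler.
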(fn `AddRuntimeSandCell`
  (params (WorldLocation :type "Vector Structure") (SurfaceNormal :type "Vector Structure"))
  (bind _sandclumps (`self.SandClumps`))
  (bind _runtimecellamount (`self.RuntimeCellAmount`))
  (bind _returnvalue (`SceneComponent.K2_GetComponentToWorld` _sandclumps))
  (bind _returnvalue_2 (`InstancedStaticMeshComponent.GetInstanceCount` _sandclumps))
  (`InstancedStaticMeshComponent.AddInstance` _sandclumps (`KismetMathLibrary.MakeTransform` (`KismetMathLibrary.InverseTransformLocation` _returnvalue (+ (* SurfaceNormal 2.0) WorldLocation)) (`KismetMathLibrary.ComposeRotators` (`KismetMathLibrary.MakeRotator` 0.0 0.0 (`KismetMathLibrary.RandomFloatInRange` 0.0 360.0)) (`KismetMathLibrary.MakeRotFromZ` (`KismetMathLibrary.InverseTransformDirection` _returnvalue SurfaceNormal)))) false)
  (set `self.CellsX` _returnvalue_2)
  (set `self.CellsY` 1)
  (set `self.MaxAmount` (* _returnvalue_2 _runtimecellamount))
  (set `self.CurrentAmount` (`KismetMathLibrary.FClamp` (+ _runtimecellamount (`self.CurrentAmount`)) 0.0 (`self.MaxAmount`))))

(fn `AddRuntimeSubstanceCell`
  (params (WorldLocation :type "Vector Structure") (SurfaceNormal :type "Vector Structure"))
  (`self.AddRuntimeSandCell` WorldLocation SurfaceNormal))

(fn `AddRuntimeSubstanceCellWithAmount`
  (params (WorldLocation :type "Vector Structure") (SurfaceNormal :type "Vector Structure") (AmountToAdd :type "Float (double-precision)"))
  (locals (PreviousMaxAmount :type "Float (double-precision)") (PreviousCurrentAmount :type "Float (double-precision)"))
  (bind _returnvalue (`KismetMathLibrary.FMax` AmountToAdd))
  (if (> _returnvalue 0.001)
    (set `local.PreviousMaxAmount` (`self.MaxAmount`))
    (set `local.PreviousCurrentAmount` (`self.CurrentAmount`))
    (`self.AddRuntimeSandCell` WorldLocation SurfaceNormal)
    (bind _output_get (set `self.MaxAmount` (+ (`local.PreviousMaxAmount`) _returnvalue)))
    (set `self.CurrentAmount` (`KismetMathLibrary.FClamp` (+ (`local.PreviousCurrentAmount`) _returnvalue) 0.0 _output_get))
    (`self.ApplyLatestRuntimeCellVisualAmount` _returnvalue)
    (return)
    (else
      (return))))

(fn `ApplyLatestRuntimeCellVisualAmount`
  (params (CellAmount :type "Float (double-precision)"))
  (locals (SafeCellAmount :type "Float (double-precision)") (SafeReferenceAmount :type "Float (double-precision)") (AmountRatio :type "Float (double-precision)") (VisualScaleFactor :type "Float (double-precision)") (LastInstanceIndex :type Integer))
  (bind (_outinstancetransform _returnvalue) (`InstancedStaticMeshComponent.GetInstanceTransform` (`self.SandClumps`) (`local.LastInstanceIndex`) false))
  (set `local.SafeCellAmount` (`KismetMathLibrary.FMax` CellAmount))
  (set `local.SafeReferenceAmount` (`KismetMathLibrary.FMax` (`self.RuntimeCellAmount`) 0.001))
  (set `local.AmountRatio` (/ (`local.SafeCellAmount`) (`local.SafeReferenceAmount`)))
  (set `local.AmountRatio` (`KismetMathLibrary.FClamp` (`local.AmountRatio`) 0.001))
  (set `local.VisualScaleFactor` (`KismetMathLibrary.MultiplyMultiply_FloatFloat` (`local.AmountRatio`) 0.45))
  (set `local.LastInstanceIndex` (- (`InstancedStaticMeshComponent.GetInstanceCount` (`self.SandClumps`)) 1))
  (if (>= (`local.LastInstanceIndex`) 0)
    (if _returnvalue
      (`InstancedStaticMeshComponent.UpdateInstanceTransform` (`self.SandClumps`) (`local.LastInstanceIndex`) (`KismetMathLibrary.MakeTransform` (.location _outinstancetransform) (.rotation _outinstancetransform) (* (.scale _outinstancetransform) (`local.VisualScaleFactor`))) false true true)
      (return)
      (else
        (return)))
    (else
      (return))))

(fn `HandleSubstanceDepleted`
  (`self.SetLifeSpan` 0.05))

(fn `UserConstructionScript`
  (`parent.UserConstructionScript`))