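; Vacuumable sand patch substance that shows its remaining amount as a pile of instanced clumps.
; The construction script sizes the interaction bounds and fills a grid with clumps, using index-based pseudo-random yaw and scale.
; Vacuuming requires a clump within radius, spawns a Niagara burst aimed at the vacuum, then defers consumption to the parent.
; Visual refresh removes clumps nearest the last interaction, within radius, toward the remaining fraction, clearing all at empty.
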(fn `ApplyVacuumInteraction`
  (params (Context :type "/Game/Systems/Substances/Core/ST_VacuumInteractionContext Structure") (`Context Vacuum Radius` :type "Float (double-precision)"))
  (returns (ConsumedAmount :type "Float (double-precision)") (Handled :type Boolean) (Completed :type Boolean))
  (`KismetSystemLibrary.PrintString` "KUM MESAJ ALDI")
  (bind _output_get (set `self.VacuumRemovalRadius` `Context Vacuum Radius`))
  (bind (_closestindex _closestdistancesquared) (`self.FindClosestSandInstanceIndex` Context_InteractionLocation_13_113903844B2C3D20C71C20B1C50859BF))
  (if (<= _closestdistancesquared (* (`self.VacuumRemovalRadius`) (`self.VacuumRemovalRadius`)))
    (bind _returnvalue (`NiagaraFunctionLibrary.SpawnSystemAtLocation` "/Game/Systems/Substances/Core/VFX/NS_SandVacuumBurst.NS_SandVacuumBurst" (.location (`InstancedStaticMeshComponent.GetInstanceTransform` (`self.SandClumps`) _closestindex true))))
    (`NiagaraComponent.SetVariablePosition` _returnvalue "User.VacuumTarget" Context_VacuumOrigin_5_64760E6245C71DF612B501BB935F7F93)
    (bind (_consumedamount _handled _completed) (`parent.ApplyVacuumInteraction` (make `/Game/Systems/Substances/Core/ST_VacuumInteractionContext` Context_SourceActor_3_FF9BA0BC40F1FF2E6C2FE09E5184D25D Context_VacuumOrigin_5_64760E6245C71DF612B501BB935F7F93 Context_InteractionLocation_13_113903844B2C3D20C71C20B1C50859BF Context_VacuumStrength_10_D2CB8D3E431B351EB7BA95B8B9CA2067 Context_DeltaTime_12_B4062DF14CF9FAFA36EA39A4C044141F) _output_get))
    (return _consumedamount _handled _completed)
    (else
      (`KismetSystemLibrary.PrintString` "MESAFE REDDETTI")
      (return 0.0 false false))))

(fn `FindClosestSandInstanceIndex`
  (params (WorldLocation :type "Vector Structure"))
  (returns (ClosestIndex :type Integer) (ClosestDistanceSquared :type "Float (double-precision)"))
  (locals (BestIndex :type Integer) (BestDistanceSquared :type "Float (double-precision)"))
  (bind _sandclumps (`self.SandClumps`))
  (set `local.BestIndex` -1)
  (set `local.BestDistanceSquared` 9999999999.0)
  (for _index (range (`InstancedStaticMeshComponent.GetInstanceCount` _sandclumps))
    (bind _returnvalue (`KismetMathLibrary.Vector_DistanceSquared` (.location (`InstancedStaticMeshComponent.GetInstanceTransform` _sandclumps _index true)) WorldLocation))
    (if (< _returnvalue (`local.BestDistanceSquared`))
      (set `local.BestDistanceSquared` _returnvalue)
      (set `local.BestIndex` _index)))
  (return (`local.BestIndex`) (`local.BestDistanceSquared`)))

(fn `RefreshSubstanceVisuals`
  (params (NewAmount :type "Float (double-precision)") (NewMaxAmount :type "Float (double-precision)"))
  (bind _sandclumps (`self.SandClumps`))
  (bind _returnvalue (- (`InstancedStaticMeshComponent.GetInstanceCount` _sandclumps) (`KismetMathLibrary.FCeil64` (* (`KismetMathLibrary.FClamp` (/ NewAmount (`KismetMathLibrary.FMax` NewMaxAmount 0.001))) (`KismetMathLibrary.Conv_IntToDouble` (* (`self.CellsY`) (`self.CellsX`)))))))
  (if (<= NewAmount 0.0001)
    (`InstancedStaticMeshComponent.ClearInstances` (`self.SandClumps`))
    (`parent.RefreshSubstanceVisuals` NewAmount NewMaxAmount)
    (else
      (if (> _returnvalue 0)
        (for _ (range _returnvalue)
          (bind (_closestindex _closestdistancesquared) (`self.FindClosestSandInstanceIndex` (`self.LastInteractionLocation`)))
          (if (<= _closestdistancesquared (* (`self.VacuumRemovalRadius`) (`self.VacuumRemovalRadius`)))
            (`InstancedStaticMeshComponent.RemoveInstance` _sandclumps _closestindex))))
      (`parent.RefreshSubstanceVisuals` NewAmount NewMaxAmount))))

(fn `UserConstructionScript`
  (bind _maxpileheight (`self.MaxPileHeight`))
  (bind _returnvalue (/ (`self.PatchSizeY`) (`self.CellsY`)))
  (bind _returnvalue_2 (/ (`self.PatchSizeX`) (`self.CellsX`)))
  (`parent.UserConstructionScript`)
  (`InstancedStaticMeshComponent.ClearInstances` (`self.SandClumps`))
  (`BoxComponent.SetBoxExtent` (`self.InteractionBounds`) (`KismetMathLibrary.MakeVector` (* (`self.PatchSizeX`) 0.5) (* (`self.PatchSizeY`) 0.5) (+ (* (`self.MaxPileHeight`) 0.5) 20.0)) true)
  (for _index (range (`self.CellsX`))
    (for _index_2 (range (`self.CellsY`))
      (`InstancedStaticMeshComponent.AddInstance` (`self.SandClumps`) (`KismetMathLibrary.MakeTransform` (`KismetMathLibrary.MakeVector` (- (* (+ (`KismetMathLibrary.Conv_IntToDouble` _index) 0.5) _returnvalue_2) (* (`self.PatchSizeX`) 0.5)) (- (* (+ (`KismetMathLibrary.Conv_IntToDouble` _index_2) 0.5) _returnvalue) (* (`self.PatchSizeY`) 0.5)) (* _maxpileheight 0.5)) (`KismetMathLibrary.MakeRotator` 0.0 0.0 (- (`KismetMathLibrary.FMod` (* _index 137.0) 360.0) 180.0)) (`KismetMathLibrary.MakeVector` (* (* (/ _returnvalue_2 100.0) 1.15) (+ (/ (`KismetMathLibrary.FMod` (* _index 73.0) 17.0) 100.0) 0.92)) (* (/ _returnvalue 100.0) 1.15) (* (/ _maxpileheight 100.0) 1.15))) false))))