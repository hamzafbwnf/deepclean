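; Prototype sand patch actor that fills a rectangular area with a grid of instanced sand clumps.
; The construction script sizes InteractionBounds to the patch and pile height, then clears and rebuilds SandClumps instances, slightly oversized so neighboring cells overlap.
; The loop counts are swapped relative to the axes they position, so the grid fits only when CellsX equals CellsY.
; It has no active runtime logic.
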(fn `UserConstructionScript`
  (bind _maxpileheight (`self.MaxPileHeight`))
  (bind _returnvalue (/ (`self.PatchSizeY`) (`self.CellsY`)))
  (bind _returnvalue_2 (/ (`self.PatchSizeX`) (`self.CellsX`)))
  (`parent.UserConstructionScript`)
  (`InstancedStaticMeshComponent.ClearInstances` (`self.SandClumps`))
  (`BoxComponent.SetBoxExtent` (`self.InteractionBounds`) (`KismetMathLibrary.MakeVector` (* (`self.PatchSizeX`) 0.5) (* (`self.PatchSizeY`) 0.5) (+ (* (`self.MaxPileHeight`) 0.5) 20.0)) true)
  (for _index (range (`self.CellsX`))
    (for _index_2 (range (`self.CellsY`))
      (`InstancedStaticMeshComponent.AddInstance` (`self.SandClumps`) (`KismetMathLibrary.MakeTransform` (`KismetMathLibrary.MakeVector` (- (* (+ (`KismetMathLibrary.Conv_IntToDouble` _index_2) 0.5) _returnvalue_2) (* (`self.PatchSizeX`) 0.5)) (- (* (+ (`KismetMathLibrary.Conv_IntToDouble` _index) 0.5) _returnvalue) (* (`self.PatchSizeY`) 0.5)) (* _maxpileheight 0.5)) (struct) (`KismetMathLibrary.MakeVector` (* (/ _returnvalue_2 100.0) 1.15) (* (/ _returnvalue 100.0) 1.15) (* (/ _maxpileheight 100.0) 1.15))) false))))