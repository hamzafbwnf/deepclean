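; Base actor for substance patches that a vacuum can remove, tracking a current amount against a maximum.
; BeginPlay clamps the starting amount into range.
; ApplyVacuumInteraction drains the amount by removal rate, vacuum strength and delta time, then reports consumed amount, handled and completed.
; It passes changes to RefreshSubstanceVisuals, an empty hook here, and prints a debug readout of the remaining amount.
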(event `self.ReceiveBeginPlay`
  (bind _output_get (set `self.MaxAmount` (`KismetMathLibrary.FMax` (`self.MaxAmount`) 0.01)))
  (set `self.CurrentAmount` (`KismetMathLibrary.FClamp` (`self.StartingAmount`) 0.0 _output_get)))

(fn `ApplyVacuumInteraction`
  (params (Context :type "/Game/Systems/Substances/Core/ST_VacuumInteractionContext Structure"))
  (returns (ConsumedAmount :type "Float (double-precision)") (Handled :type Boolean) (Completed :type Boolean))
  (locals (OldAmount :type "Float (double-precision)") (RequestedRemoval :type "Float (double-precision)"))
  (bind _currentamount (`self.CurrentAmount`))
  (bind _returnvalue (* (`self.RemovalRate`) (* (`KismetMathLibrary.FMax` Context_VacuumStrength_10_D2CB8D3E431B351EB7BA95B8B9CA2067) (`KismetMathLibrary.FMax` Context_DeltaTime_12_B4062DF14CF9FAFA36EA39A4C044141F))))
  (set `local.RequestedRemoval` _returnvalue)
  (if (and (and (`self.CanBeRemoved`) (> _returnvalue 0.0)) (> (`self.CurrentAmount`) 0.0))
    (set `local.OldAmount` _currentamount)
    (bind _output_get (set `self.CurrentAmount` (`KismetMathLibrary.FClamp` (- _currentamount (`local.RequestedRemoval`)) 0.0 (`self.MaxAmount`))))
    (`self.RefreshSubstanceVisuals` _output_get (`self.MaxAmount`))
    (`KismetSystemLibrary.PrintString` (`KismetTextLibrary.Conv_TextToString` (`|FormatText` "Substance: {Current} / {Maximum}" (`self.CurrentAmount`) (`self.MaxAmount`))))
    (return (- (`local.OldAmount`) (`self.CurrentAmount`)) true (<= (`self.CurrentAmount`) 0.001))
    (else
      (return 0.0 (`self.CanBeRemoved`) (<= (`self.CurrentAmount`) 0.001)))))

(fn `RefreshSubstanceVisuals`
  (params (NewAmount :type "Float (double-precision)") (NewMaxAmount :type "Float (double-precision)")))

(fn `UserConstructionScript`)