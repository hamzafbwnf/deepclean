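; BP_SludgePatch is a substance patch that shows its sludge amount as a flat surface growing and shrinking in the world.
; The construction script, BeginPlay and RefreshSubstanceVisuals extend the parent and pass starting, current or new amounts to ApplySludgeVisualAmount.
; That function keeps one SludgeSurface instance, removed when nearly empty.
; Its XY scale lerps between minimum and maximum by square root of the fill ratio, so area roughly tracks amount.
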(event `self.RefreshSubstanceVisuals`
  (params (NewAmount :type "Float (double-precision)") (NewMaxAmount :type "Float (double-precision)"))
  (`parent.RefreshSubstanceVisuals` NewAmount NewMaxAmount)
  (`self.ApplySludgeVisualAmount` NewAmount NewMaxAmount))

(event `self.ReceiveBeginPlay`
  (`parent.ReceiveBeginPlay`)
  (`self.ApplySludgeVisualAmount` (`self.CurrentAmount`) (`self.MaxAmount`)))

(fn `ApplySludgeVisualAmount`
  (params (VisualAmount :type "Float (double-precision)") (VisualMaxAmount :type "Float (double-precision)"))
  (bind _sludgesurface (`self.SludgeSurface`))
  (bind _returnvalue (`KismetMathLibrary.Lerp` (`self.SludgeMinimumVisualScale`) (`self.SludgeMaximumVisualScale`) (`KismetMathLibrary.Sqrt` (`KismetMathLibrary.FClamp` (/ VisualAmount (`KismetMathLibrary.FMax` VisualMaxAmount 0.001))))))
  (bind _returnvalue_2 (`KismetMathLibrary.MakeTransform` (`KismetMathLibrary.MakeVector` 0.0) (`KismetMathLibrary.MakeRotator` 0.0) (`KismetMathLibrary.MakeVector` _returnvalue _returnvalue 1.0)))
  (if (> VisualAmount 0.001)
    (if (> (`InstancedStaticMeshComponent.GetInstanceCount` _sludgesurface) 0)
      (`InstancedStaticMeshComponent.UpdateInstanceTransform` _sludgesurface 0 _returnvalue_2 false true true)
      (else
        (`InstancedStaticMeshComponent.AddInstance` _sludgesurface _returnvalue_2 false)))
    (elif (> (`InstancedStaticMeshComponent.GetInstanceCount` _sludgesurface) 0)
      (`InstancedStaticMeshComponent.RemoveInstance` _sludgesurface 0))))

(fn `UserConstructionScript`
  (`parent.UserConstructionScript`)
  (`self.ApplySludgeVisualAmount` (`self.StartingAmount`) (`self.MaxAmount`)))