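; Runtime-created sludge patch, a substance actor that holds an amount of sludge and takes part in flow through BP_SludgeFlowManager.
; Adding sludge grows both current and max amount, updates visuals and registers with the manager; EndPlay unregisters.
; It exposes flow state plus clamped extract and restore functions, while vacuum interaction always reports unhandled.
; Depletion sets a short lifespan for self-destruction, which adding or restoring sludge cancels.
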(event `self.ApplyLatestRuntimeCellVisualAmount`
  (params (CellAmount :type "Float (double-precision)"))
  (`self.ApplySludgeVisualAmount` CellAmount (`self.MaxAmount`))
  (`self.EnsureSludgeFlowRegistration`))

(event `self.AddRuntimeSubstanceCellWithAmount`
  (params (WorldLocation :type "Vector Structure") (SurfaceNormal :type "Vector Structure") (AmountToAdd :type "Float (double-precision)"))
  (bind _returnvalue (`KismetMathLibrary.FMax` AmountToAdd))
  (bind _returnvalue_2 (+ (`self.MaxAmount`) _returnvalue))
  (if (> _returnvalue 0.001)
    (`self.SetLifeSpan` 0.0)
    (set `self.MaxAmount` _returnvalue_2)
    (bind _output_get (set `self.CurrentAmount` (`KismetMathLibrary.FClamp` (+ (`self.CurrentAmount`) _returnvalue) 0.0 _returnvalue_2)))
    (`self.ApplyLatestRuntimeCellVisualAmount` _output_get)))

(event `self.ReceiveBeginPlay`
  (`parent.ReceiveBeginPlay`))

(event `self.ReceiveActorBeginOverlap`
  (params (OtherActor :type "Actor Object Reference"))
  (`parent.ReceiveActorBeginOverlap` OtherActor))

(event `self.ReceiveTick`
  (params (DeltaSeconds :type "Float (single-precision)"))
  (`parent.ReceiveTick` DeltaSeconds))

(event `self.HandleSubstanceDepleted`
  (`parent.HandleSubstanceDepleted`)
  (`self.SetLifeSpan` 0.05))

(event `self.ReceiveEndPlay`
  (params (EndPlayReason :type "EEndPlayReason Enum" :default "Destroyed"))
  (`parent.ReceiveEndPlay` EndPlayReason)
  (message `/Game/Systems/Substances/Sludge/Flow/BPI_SludgeFlowManager.UnregisterSludgePatch` (`self.CachedSludgeFlowManager`) self))

(fn `ApplyVacuumInteraction`
  (params (Context :type "/Game/Systems/Substances/Core/ST_VacuumInteractionContext Structure") (`Context Vacuum Radius` :type "Float (double-precision)"))
  (returns (ConsumedAmount :type "Float (double-precision)") (Handled :type Boolean) (Completed :type Boolean) (ConsumedSubstanceType :type "/Game/Systems/Substances/Core/E_SubstanceType Enum"))
  (return 0.0 false false "NewEnumerator0"))

(fn `EnsureSludgeFlowRegistration`
  (bind _cachedsludgeflowmanager (`self.CachedSludgeFlowManager`))
  (`/Engine/EditorBlueprintResources/StandardMacros.IsValid` _cachedsludgeflowmanager
    (:`Is Valid`
      (message `/Game/Systems/Substances/Sludge/Flow/BPI_SludgeFlowManager.RegisterSludgePatch` _cachedsludgeflowmanager self))
    (:`Is Not Valid`
      (bind _returnvalue (`GameplayStatics.GetActorOfClass` "/Game/Systems/Substances/Sludge/Flow/BP_SludgeFlowManager.BP_SludgeFlowManager_C"))
      (`/Engine/EditorBlueprintResources/StandardMacros.IsValid` _returnvalue
        (:`Is Valid`
          (set `self.CachedSludgeFlowManager` _returnvalue)
          (message `/Game/Systems/Substances/Sludge/Flow/BPI_SludgeFlowManager.RegisterSludgePatch` _returnvalue self))))))

(fn `GetSludgeFlowState`
  (returns (CurrentAmount :type "Float (double-precision)") (WorldLocation :type "Vector Structure") (SurfaceNormal :type "Vector Structure") (bCanFlow :type Boolean))
  (bind _currentamount (`self.CurrentAmount`))
  (return _currentamount (`self.K2_GetActorLocation` self) (`self.GetActorUpVector` self) (> _currentamount 0.001)))

(fn `RestoreSludgeAmount`
  (params (AmountToRestore :type "Float (double-precision)"))
  (returns (RestoredAmount :type "Float (double-precision)"))
  (locals (Local_RestoredAmount :type "Float (double-precision)"))
  (bind _currentamount (`self.CurrentAmount`))
  (bind _maxamount (`self.MaxAmount`))
  (bind _local_restoredamount (`local.Local_RestoredAmount`))
  (set `local.Local_RestoredAmount` (`KismetMathLibrary.FClamp` AmountToRestore 0.0 (`KismetMathLibrary.FMax` (- _maxamount (`KismetMathLibrary.FMax` _currentamount)))))
  (if (> _local_restoredamount 0.0)
    (`self.SetLifeSpan` self 0.0)
    (bind _output_get (set `self.CurrentAmount` (`KismetMathLibrary.FClamp` (+ _currentamount _local_restoredamount) 0.0 _maxamount)))
    (`self.RefreshSubstanceVisuals` _output_get _maxamount)
    (return _local_restoredamount)
    (else
      (return _local_restoredamount))))

(fn `TryExtractSludgeAmount`
  (params (RequestedAmount :type "Float (double-precision)"))
  (returns (ExtractedAmount :type "Float (double-precision)"))
  (locals (Local_ExtractedAmount :type "Float (double-precision)"))
  (bind _currentamount (`self.CurrentAmount`))
  (bind _local_extractedamount (`local.Local_ExtractedAmount`))
  (bind _maxamount (`self.MaxAmount`))
  (set `local.Local_ExtractedAmount` (`KismetMathLibrary.FClamp` RequestedAmount 0.0 (`KismetMathLibrary.FMax` _currentamount)))
  (bind _output_get (set `self.CurrentAmount` (`KismetMathLibrary.FClamp` (- _currentamount _local_extractedamount) 0.0 _maxamount)))
  (`self.RefreshSubstanceVisuals` _output_get _maxamount)
  (if (and (> _local_extractedamount 0.0) (<= _output_get 0.001))
    (`self.HandleSubstanceDepleted`)
    (return _local_extractedamount)
    (else
      (return _local_extractedamount))))

(fn `UserConstructionScript`
  (`parent.UserConstructionScript`))