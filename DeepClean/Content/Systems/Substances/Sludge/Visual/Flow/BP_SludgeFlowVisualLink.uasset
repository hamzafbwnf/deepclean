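; Visual link actor that draws a sludge flow between a source and target as a chain of oriented decal segments.
; ConfigureFlowPath rebuilds it on first use, target movement beyond a threshold or support change, building segments only for same-surface links.
; That branch runs both the interpolated same-surface builder, whose alphas divide by zero, and a cross-surface builder using vertical traces.
; Each decal's dynamic material receives the surface normal; EndPlay clears all segments.
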(event `self.ReceiveEndPlay`
  (params (EndPlayReason :type "EEndPlayReason Enum" :default "Destroyed"))
  (`self.ClearFlowSegments`))

(fn `BuildCrossSurfacePath`
  (params (SourceLocation :type "Vector Structure") (TargetLocation :type "Vector Structure"))
  (bind _returnvalue (`KismetMathLibrary.MakeVector` 0.0 0.0 (* (`self.SegmentLength`) 0.6)))
  (for _index (range (+ (- (`self.MaxSegments`) 1) 1))
    (bind _returnvalue_2 (`KismetMathLibrary.VLerp` SourceLocation TargetLocation (/ (`KismetMathLibrary.Conv_IntToDouble` _index) (`KismetMathLibrary.Conv_IntToDouble` (`self.MaxSegments`)))))
    (bind (_outhit _returnvalue_3) (`KismetSystemLibrary.LineTraceSingle` (+ _returnvalue_2 (`KismetMathLibrary.MakeVector` 0.0 0.0 100.0)) (+ _returnvalue_2 (`KismetMathLibrary.MakeVector` 0.0 0.0 -100.0)) "TraceTypeQuery1"))
    (if _returnvalue_3
      (bind (_bblockinghit _binitialoverlap _time _distance _location _impactpoint _normal _impactnormal) (`GameplayStatics.BreakHitResult` _outhit))
      (bind _returnvalue_4 (+ _impactpoint _impactnormal))
      (`self.CreateFlowSegment` (+ _returnvalue_4 _returnvalue) (- _returnvalue_4 _returnvalue) _impactnormal _index))))

(fn `BuildSameSurfacePath`
  (params (SourceLocation :type "Vector Structure") (TargetLocation :type "Vector Structure") (SourceNormal :type "Vector Structure") (TargetNormal :type "Vector Structure"))
  (bind _returnvalue (`KismetMathLibrary.Conv_IntToDouble` 0))
  (`self.ClearFlowSegments`)
  (for _index (range (+ (- (`KismetMathLibrary.Clamp` (`KismetMathLibrary.Conv_Int64ToInt` (`KismetMathLibrary.FCeil64` (/ (`KismetMathLibrary.Vector_Distance` SourceLocation TargetLocation) (`self.SegmentLength`)))) 1 (`self.MaxSegments`)) 1) 1))
    (bind _returnvalue_2 (`KismetMathLibrary.Conv_IntToDouble` _index))
    (bind _returnvalue_3 (/ (+ _returnvalue_2 1.0) _returnvalue))
    (`self.CreateFlowSegment` (`KismetMathLibrary.VLerp` SourceLocation TargetLocation (/ _returnvalue_2 _returnvalue)) (`KismetMathLibrary.VLerp` SourceLocation TargetLocation _returnvalue_3) (`KismetMathLibrary.Normal` (`KismetMathLibrary.VLerp` SourceNormal TargetNormal _returnvalue_3)) _index)))

(fn `ClearFlowSegments`
  (for _array_element (`self.SegmentDecals`)
    (`/Engine/EditorBlueprintResources/StandardMacros.IsValid` _array_element
      (:`Is Valid`
        (`ActorComponent.K2_DestroyComponent` _array_element))))
  (`KismetArrayLibrary.Array_Clear` (`self.SegmentDecals`))
  (set `self.bPathInitialized` false))

(fn `ConfigureFlowPath`
  (params (SourceLocation :type "Vector Structure") (TargetLocation :type "Vector Structure") (SourceNormal :type "Vector Structure") (TargetNormal :type "Vector Structure") (bSameSupportSurface :type Boolean))
  (if (or (or (not (`self.bPathInitialized`)) (> (`KismetMathLibrary.VSize` (- TargetLocation (`self.LastTargetLocation`))) (`self.RebuildDistance`))) (!= bSameSupportSurface (`self.bLastSameSupport`)))
    (`self.ClearFlowSegments`)
    (set `self.LastSourceLocation` SourceLocation)
    (set `self.LastTargetLocation` TargetLocation)
    (set `self.bLastSameSupport` bSameSupportSurface)
    (set `self.bPathInitialized` true)
    (if bSameSupportSurface
      (`self.BuildSameSurfacePath` SourceLocation TargetLocation SourceNormal TargetNormal)
      (`self.BuildCrossSurfacePath` SourceLocation TargetLocation))))

(fn `CreateFlowSegment`
  (params (SegmentStart :type "Vector Structure") (SegmentEnd :type "Vector Structure") (SurfaceNormal :type "Vector Structure") (SegmentIndex :type Integer))
  (bind _returnvalue (`KismetMathLibrary.Normal` SurfaceNormal))
  (bind _returnvalue_2 (- SegmentEnd SegmentStart))
  (bind _returnvalue_3 (`KismetMathLibrary.VSize` _returnvalue_2))
  (bind _returnvalue_4 (`KismetMathLibrary.Normal` _returnvalue_2))
  (if (> _returnvalue_3 1.0)
    (bind _returnvalue_5 (`GameplayStatics.SpawnDecalAtLocation` (`self.FlowMaterial`) (`KismetMathLibrary.MakeVector` (`self.ProjectionDepth`) (`self.SegmentWidth`) (`KismetMathLibrary.FMax` (* _returnvalue_3 0.5) 1.0)) (`KismetMathLibrary.VLerp` SegmentStart SegmentEnd 0.5) (`KismetMathLibrary.MakeRotationFromAxes` (- (0.0 0.0 0.0) _returnvalue) (`KismetMathLibrary.Normal` (`KismetMathLibrary.Cross_VectorVector` _returnvalue _returnvalue_4)) _returnvalue_4)))
    (`/Engine/EditorBlueprintResources/StandardMacros.IsValid` _returnvalue_5
      (:`Is Valid`
        (bind _returnvalue_6 (`DecalComponent.CreateDynamicMaterialInstance` _returnvalue_5))
        (`MaterialInstanceDynamic.SetVectorParameterValueByInfo` _returnvalue_6 (make `MaterialParameterInfo` "ProjectionNormalWS") (`KismetMathLibrary.Conv_VectorToLinearColor` _returnvalue))
        (`KismetArrayLibrary.Array_Add` (`self.SegmentDecals`) _returnvalue_5)))))

(fn `UserConstructionScript`)