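; Manager actor that makes registered sludge patches flow downhill across surfaces.
; A looping timer processes a limited round-robin batch, tracing down from one cell along each sloped patch's downhill direction to find a target.
; Transfers extract sludge, deposit it through a service component found on the player pawn, and refund any uncommitted amount.
; Patches communicate through an interface, and the active-cell cap limits both registration and flow.
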(event `self.ReceiveBeginPlay`
  (bind _returnvalue (`KismetMathLibrary.FMax` (`self.FlowInterval`) 0.05))
  (`parent.ReceiveBeginPlay`)
  (if (`self.bEnableSludgeFlow`)
    (`KismetSystemLibrary.K2_SetTimer` self "ProcessSludgeFlowBatch" _returnvalue true false _returnvalue 0.0)))

(event `/Game/Systems/Substances/Sludge/Flow/BPI_SludgeFlowManager.UnregisterSludgePatch`
  (params (PatchActor :type "Actor Object Reference"))
  (`KismetArrayLibrary.Array_RemoveItem` (`self.RegisteredSludgePatches`) PatchActor)
  (`KismetArrayLibrary.Array_RemoveItem` (`self.ActiveFlowQueue`) PatchActor))

(fn `EnsureSludgeFlowService`
  (bind _returnvalue (`GameplayStatics.GetPlayerPawn` 0))
  (bind _returnvalue_2 (`self.GetComponentsByInterface` _returnvalue "/Game/Systems/Substances/Sludge/Flow/BPI_SludgeFlowService.BPI_SludgeFlowService_C"))
  (`/Engine/EditorBlueprintResources/StandardMacros.IsValid` (`self.CachedSludgeFlowService`)
    (:`Is Not Valid`
      (`/Engine/EditorBlueprintResources/StandardMacros.IsValid` _returnvalue
        (:`Is Valid`
          (if (> (`KismetArrayLibrary.Array_Length` _returnvalue_2) 0)
            (set `self.CachedSludgeFlowService` (`|GetArrayItem` _returnvalue_2))))))))

(fn `ExecuteSludgeTransfer`
  (params (SourcePatch :type "Actor Object Reference") (TargetWorldLocation :type "Vector Structure") (TargetSurfaceNormal :type "Vector Structure") (TargetSurfaceOwner :type "Actor Object Reference") (TargetSupportComponent :type "PrimitiveComponent Object Reference") (RequestedAmount :type "Float (double-precision)"))
  (returns (ExtractedAmount :type "Float (double-precision)") (CommittedAmount :type "Float (double-precision)") (RestoredAmount :type "Float (double-precision)") (ResultPatch :type "Actor Object Reference") (bTransferred :type Boolean))
  (locals (Local_ExtractedAmount :type "Float (double-precision)") (Local_CommittedAmount :type "Float (double-precision)") (Local_ResultPatch :type "Actor Object Reference") (Local_bDeposited :type Boolean) (Local_RefundRequested :type "Float (double-precision)") (Local_RestoredAmount :type "Float (double-precision)"))
  (bind _local_resultpatch (`local.Local_ResultPatch`))
  (bind _local_extractedamount (`local.Local_ExtractedAmount`))
  (bind _local_extractedamount_2 (`local.Local_ExtractedAmount`))
  (bind _local_committedamount (`local.Local_CommittedAmount`))
  (bind _returnvalue (`KismetMathLibrary.FMax` (- _local_extractedamount _local_committedamount)))
  (bind _returnvalue_2 (and (`local.Local_bDeposited`) (> _local_committedamount 0.001)))
  (`/Engine/EditorBlueprintResources/StandardMacros.IsValid` SourcePatch
    (:`Is Valid`
      (if (and true (`KismetSystemLibrary.DoesImplementInterface` SourcePatch "/Game/Systems/Substances/Sludge/Flow/BPI_SludgeFlowPatch.BPI_SludgeFlowPatch_C"))
        (bind _extractedamount (message `/Game/Systems/Substances/Sludge/Flow/BPI_SludgeFlowPatch.TryExtractSludgeAmount` SourcePatch RequestedAmount))
        (set `local.Local_ExtractedAmount` _extractedamount)
        (if (> _local_extractedamount 0.001)
          (bind (_committedamount _resultpatch _bdeposited) (`self.RequestSludgeDepositThroughService` TargetWorldLocation TargetSurfaceNormal TargetSurfaceOwner TargetSupportComponent _local_extractedamount))
          (set `local.Local_CommittedAmount` _committedamount)
          (set `local.Local_ResultPatch` _resultpatch)
          (set `local.Local_bDeposited` _bdeposited)
          (set `local.Local_RefundRequested` _returnvalue)
          (if (> (`local.Local_RefundRequested`) 0.001)
            (bind _restoredamount (message `/Game/Systems/Substances/Sludge/Flow/BPI_SludgeFlowPatch.RestoreSludgeAmount` SourcePatch _returnvalue))
            (set `local.Local_RestoredAmount` _restoredamount)
            (return _local_extractedamount_2 _local_committedamount (`local.Local_RestoredAmount`) _local_resultpatch _returnvalue_2)
            (else
              (return _local_extractedamount_2 _local_committedamount 0.0 _local_resultpatch _returnvalue_2)))
          (else
            (return _local_extractedamount_2 0.0 0.0 null false)))
        (else
          (return 0.0 0.0 0.0 null false))))
    (:`Is Not Valid`
      (return 0.0 0.0 0.0 null false))))

(fn `ProcessSludgeFlowBatch`
  (locals (Local_BatchStartCount :type Integer) (Local_CellsToProcess :type Integer) (Local_CurrentAmount :type "Float (double-precision)") (Local_SourceNormal :type "Vector Structure") (Local_bCanFlow :type Boolean) (Local_SourcePatch :type "Actor Object Reference") (Local_SourceLocation :type "Vector Structure"))
  (bind _registeredsludgepatches (`self.RegisteredSludgePatches`))
  (bind _local_currentamount (`local.Local_CurrentAmount`))
  (bind _mintransferamount (`self.MinTransferAmount`))
  (bind _local_cellstoprocess (`local.Local_CellsToProcess`))
  (bind _returnvalue (`KismetArrayLibrary.Array_Length` _registeredsludgepatches))
  (bind _returnvalue_2 (`KismetArrayLibrary.Array_Length` _registeredsludgepatches))
  (bind _returnvalue_3 (mod (`self.CurrentQueueIndex`) _returnvalue_2))
  (if (`self.bEnableSludgeFlow`)
    (set `local.Local_BatchStartCount` _returnvalue)
    (set `local.Local_CellsToProcess` (`KismetMathLibrary.Min` (`KismetMathLibrary.Max` (`self.MaxCellsPerBatch`)) _returnvalue))
    (if (> _local_cellstoprocess 0)
      (set `self.FlowEpoch` (+ (`self.FlowEpoch`) 1))
      (for _ (range _local_cellstoprocess)
        (if (> _returnvalue_2 0)
          (bind _output_get (set `local.Local_SourcePatch` (`|GetArrayItem` _registeredsludgepatches _returnvalue_3)))
          (set `self.CurrentQueueIndex` (mod (+ _returnvalue_3 1) _returnvalue_2))
          (if (and (`KismetSystemLibrary.IsValid` _output_get) (`KismetSystemLibrary.DoesImplementInterface` _output_get "/Game/Systems/Substances/Sludge/Flow/BPI_SludgeFlowPatch.BPI_SludgeFlowPatch_C"))
            (bind (_currentamount _worldlocation _surfacenormal _bcanflow) (message `/Game/Systems/Substances/Sludge/Flow/BPI_SludgeFlowPatch.GetSludgeFlowState` _output_get))
            (set `local.Local_CurrentAmount` _currentamount)
            (set `local.Local_SourceLocation` _worldlocation)
            (set `local.Local_SourceNormal` _surfacenormal)
            (set `local.Local_bCanFlow` _bcanflow)
            (if (and (and (`local.Local_bCanFlow`) (> _local_currentamount _mintransferamount)) (< _returnvalue_2 (`self.MaxActiveCells`)))
              (bind (_targetworldlocation _targetsurfacenormal _targetsurfaceowner _targetsupportcomponent _bfoundtarget) (`self.ResolveDownhillFlowTarget` _output_get (`local.Local_SourceLocation`) (`local.Local_SourceNormal`)))
              (if _bfoundtarget
                (`self.ExecuteSludgeTransfer` _output_get _targetworldlocation _targetsurfacenormal _targetsurfaceowner _targetsupportcomponent (`KismetMathLibrary.FMin` _local_currentamount (`KismetMathLibrary.FMax` (* (`self.MaxTransferAmountPerStep`) (`KismetMathLibrary.FMax` (- (`KismetMathLibrary.FClamp` (`self.Viscosity`)) 1.0) 0.05)) _mintransferamount)))))))))))

(fn `RegisterSludgePatch`
  (params (PatchActor :type "Actor Object Reference"))
  (returns (bRegistered :type Boolean))
  (locals (Local_bRegistered :type Boolean))
  (bind _registeredsludgepatches (`self.RegisteredSludgePatches`))
  (`/Engine/EditorBlueprintResources/StandardMacros.IsValid` PatchActor
    (:`Is Valid`
      (if (`KismetSystemLibrary.DoesImplementInterface` PatchActor "/Game/Systems/Substances/Sludge/Flow/BPI_SludgeFlowPatch.BPI_SludgeFlowPatch_C")
        (if (`KismetArrayLibrary.Array_Contains` _registeredsludgepatches PatchActor)
          (set `local.Local_bRegistered` true)
          (elif (not (>= (`KismetArrayLibrary.Array_Length` _registeredsludgepatches) (`self.MaxActiveCells`)))
            (`KismetArrayLibrary.Array_AddUnique` _registeredsludgepatches PatchActor)
            (set `local.Local_bRegistered` true)))))
    (:`Is Not Valid`
      _))
  (return (`local.Local_bRegistered`)))

(fn `RequestSludgeDepositThroughService`
  (params (WorldLocation :type "Vector Structure") (SurfaceNormal :type "Vector Structure") (SurfaceOwner :type "Actor Object Reference") (SupportComponent :type "PrimitiveComponent Object Reference") (RequestedAmount :type "Float (double-precision)"))
  (returns (CommittedAmount :type "Float (double-precision)") (ResultPatch :type "Actor Object Reference") (bDeposited :type Boolean))
  (bind _cachedsludgeflowservice (`self.CachedSludgeFlowService`))
  (`self.EnsureSludgeFlowService`)
  (`/Engine/EditorBlueprintResources/StandardMacros.IsValid` _cachedsludgeflowservice
    (:`Is Valid`
      (bind (_committedamount _resultpatch _bdeposited) (message `/Game/Systems/Substances/Sludge/Flow/BPI_SludgeFlowService.RequestSludgeFlowDeposit` _cachedsludgeflowservice WorldLocation SurfaceNormal SurfaceOwner SupportComponent RequestedAmount))
      (return _committedamount _resultpatch _bdeposited))
    (:`Is Not Valid`
      (return 0.0 null false))))

(fn `ResolveDownhillFlowTarget`
  (params (SourcePatch :type "Actor Object Reference") (SourceLocation :type "Vector Structure") (SourceSurfaceNormal :type "Vector Structure"))
  (returns (TargetWorldLocation :type "Vector Structure") (TargetSurfaceNormal :type "Vector Structure") (TargetSurfaceOwner :type "Actor Object Reference") (TargetSupportComponent :type "PrimitiveComponent Object Reference") (bFoundTarget :type Boolean))
  (bind _returnvalue (`KismetMathLibrary.Normal` SourceSurfaceNormal))
  (bind _returnvalue_2 (`KismetMathLibrary.MakeVector` 0.0 0.0 -1.0))
  (bind _returnvalue_3 (`KismetMathLibrary.ProjectVectorOnToPlane` _returnvalue_2 _returnvalue))
  (bind _returnvalue_4 (+ (+ SourceLocation (* (`KismetMathLibrary.Normal` _returnvalue_3) (`KismetMathLibrary.FMax` (`self.CellSpacing`) 1.0))) (* _returnvalue (`self.FlowTraceStartOffset`))))
  (if (> (`KismetMathLibrary.VSize` _returnvalue_3) (`KismetMathLibrary.Sin` (`KismetMathLibrary.DegreesToRadians` (`self.MinSlopeAngle`))))
    (bind (_outhit _returnvalue_5) (`KismetSystemLibrary.LineTraceSingle` _returnvalue_4 (+ _returnvalue_4 (* _returnvalue_2 (`self.FlowTraceDepth`))) "TraceTypeQuery1" false (`|MakeArray` SourcePatch)))
    (if _returnvalue_5
      (bind (_bblockinghit _binitialoverlap _time _distance _location _impactpoint _normal _impactnormal _physmat _hitactor _hitcomponent) (`GameplayStatics.BreakHitResult` _outhit))
      (return _impactpoint _impactnormal _hitactor _hitcomponent true)
      (else
        (return (0.0 0.0 0.0) (0.0 0.0 0.0) null null false)))
    (else
      (return (0.0 0.0 0.0) (0.0 0.0 0.0) null null false))))

(fn `UserConstructionScript`)