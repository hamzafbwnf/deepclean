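; BP_KelpSpawner scatters kelp over the ground within a box volume when play begins.
; BeginPlay fires repeated downward visibility traces at random points in the box, between fixed world heights, adding a KelpInstances instance slightly above each hit.
; The construction script fits an orthographic Kelpcamera to the box's larger horizontal extent and writes its width and location to the MPC_Radar parameter collection.
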(event `self.ReceiveBeginPlay`
  (bind (_origin _boxextent) (`KismetSystemLibrary.GetComponentBounds` (`self.Box`)))
  (bind (_returnvalue_x _returnvalue_y) (`KismetMathLibrary.BreakVector` (`KismetMathLibrary.RandomPointInBoundingBox` _origin _boxextent)))
  (for _ (range 1 76)
    (bind (_outhit _returnvalue) (`KismetSystemLibrary.LineTraceSingle` (`KismetMathLibrary.MakeVector` _returnvalue_x _returnvalue_y 100.0) (`KismetMathLibrary.MakeVector` _returnvalue_x _returnvalue_y -1000.0) "TraceTypeQuery1"))
    (if _returnvalue
      (`InstancedStaticMeshComponent.AddInstance` (`self.KelpInstances`) (`KismetMathLibrary.MakeTransform` (`KismetMathLibrary.MakeVector` (.x (`.Location` (`GameplayStatics.BreakHitResult` _outhit))) (.y (`.Location` (`GameplayStatics.BreakHitResult` _outhit))) (+ (.z (`.Location` (`GameplayStatics.BreakHitResult` _outhit))) 100.0))) true))))

(fn `UserConstructionScript`
  (bind _kelpcamera (`self.kelpcamera`))
  (bind (_origin _boxextent) (`KismetSystemLibrary.GetComponentBounds` (`self.Box`)))
  (bind _returnvalue (* (`KismetMathLibrary.FMax` (.x _boxextent) (.y _boxextent)) 2.0))
  (set `SceneCaptureComponent2D.OrthoWidth` _returnvalue _kelpcamera)
  (`KismetMaterialLibrary.SetScalarParameterValue` "/Game/kelp/kelp/StaticMeshes/MPC_Radar.MPC_Radar" "KameraOrthoGenislik" _returnvalue)
  (`KismetMaterialLibrary.SetVectorParameterValue` "/Game/kelp/kelp/StaticMeshes/MPC_Radar.MPC_Radar" "KameraLokasyonu" (`KismetMathLibrary.Conv_VectorToLinearColor` (`SceneComponent.K2_GetComponentLocation` _kelpcamera))))