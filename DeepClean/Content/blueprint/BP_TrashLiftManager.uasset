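; Manager that lifts trash by pushing registered physics components along a lift direction.
; Register and unregister functions keep a reference count per component in a map, so a component stays active until its last registration is released.
; A looping timer started on BeginPlay applies velocity-change impulses scaled by acceleration and update interval to simulating components, and attempts to drop invalid entries.
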(event `self.ReceiveBeginPlay`
  (`KismetSystemLibrary.K2_SetTimerDelegate` (delegate `ApplyTrashLift`) (`self.UpdateInterval`) true true))

(event `ApplyTrashLift`
  (bind _activeliftcomponents (`self.ActiveLiftComponents`))
  (bind _keys (`BlueprintMapLibrary.Map_Keys` _activeliftcomponents))
  (for _array_element _keys
    (`/Engine/EditorBlueprintResources/StandardMacros.IsValid` _array_element
      (:`Is Valid`
        (if (`SceneComponent.IsSimulatingPhysics` _array_element "None")
          (`PrimitiveComponent.AddImpulse` _array_element (* (`self.LiftDirection`) (* (`self.LiftAcceleration`) (`self.UpdateInterval`))) "None" true)
          (`/Engine/EditorBlueprintResources/StandardMacros.DoOnce` false)))
      (:`Is Not Valid`
        (`BlueprintMapLibrary.Map_Remove` _activeliftcomponents)))))

(fn `RegisterLiftComponent`
  (params (LiftComponent :type "PrimitiveComponent Object Reference"))
  (bind _activeliftcomponents (`self.ActiveLiftComponents`))
  (bind (_value _returnvalue) (`BlueprintMapLibrary.Map_Find` _activeliftcomponents LiftComponent))
  (`/Engine/EditorBlueprintResources/StandardMacros.IsValid` LiftComponent
    (:`Is Valid`
      (if (`SceneComponent.IsSimulatingPhysics` LiftComponent "None")
        (if _returnvalue
          (`BlueprintMapLibrary.Map_Add` _activeliftcomponents LiftComponent (+ _value 1))
          (else
            (`BlueprintMapLibrary.Map_Add` _activeliftcomponents LiftComponent 1)))))))

(fn `UnregisterLiftComponent`
  (params (LiftComponent :type "PrimitiveComponent Object Reference"))
  (bind _activeliftcomponents (`self.ActiveLiftComponents`))
  (bind (_value _returnvalue) (`BlueprintMapLibrary.Map_Find` _activeliftcomponents LiftComponent))
  (if _returnvalue
    (if (> _value 1)
      (`BlueprintMapLibrary.Map_Add` _activeliftcomponents LiftComponent (- _value 1))
      (else
        (`BlueprintMapLibrary.Map_Remove` _activeliftcomponents LiftComponent)))))

(fn `UserConstructionScript`)