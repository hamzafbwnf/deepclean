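; BP_MasterTrash is a trash actor, apparently the base class, that can be flagged as being vacuumed.
; Its only live logic is SetVacuumState, which stores the IsBeingVacuumed flag; BeginPlay, Tick and the construction script are empty.
; Disconnected leftover chains would nudge it while toggling distance field lighting, write its location to the MPC_Radar parameter collection, or apply randomly delayed, timeline-driven bobbing force.
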(event `self.ReceiveBeginPlay`)

(event `self.ReceiveTick`
  (params (DeltaSeconds :type "Float (single-precision)")))

(event `/Game/blueprint/BPI_Interactable.SetVacuumState`
  (params (State :type Boolean))
  (set `self.IsBeingVacuumed` State))

(fn `UserConstructionScript`)