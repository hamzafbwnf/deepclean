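; Water current volume that pushes physics-simulating components inside its box and adds periodic upward wave surges.
; Timers re-roll target strength, trigger surges and apply frequent impulses along a sine/cosine-driven direction, drawing a debug arrow.
; Surge decay and direction updates run inside the per-component loop, so they depend on what is in the box.
; Tick eases strength toward its target and feeds intensity, speed and an accumulated caustics offset to the MPC_Radar parameter collection.
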(event `self.ReceiveBeginPlay`
  (`|ExecutionSequence`
    (:`then_0`
      (`KismetSystemLibrary.K2_SetTimerDelegate` (delegate `Set Current Strength`) 3.0 true)
      (`self.Set Current Strength`)
      (`KismetSystemLibrary.K2_SetTimerDelegate` (delegate `TriggerWaveSurge`) 15.0 true))
    (:`then_1`
      (`KismetSystemLibrary.K2_SetTimerDelegate` (delegate `ApplyCurrentForces`) 0.05 true))))

(event `TriggerWaveSurge`
  (set `self.Z_WaveSurge` 3500.0)
  (`KismetSystemLibrary.PrintString` "Dalga başladı")
  (set `self.IsWaveActive` true))

(event `Set Current Strength`
  (set `self.TargetStrength` (`KismetMathLibrary.RandomFloatInRange` 200.0 1500.0)))

(event `ApplyCurrentForces`
  (bind _returnvalue (`self.K2_GetActorLocation`))
  (bind _returnvalue_2 (`GameplayStatics.GetTimeSeconds`))
  (for _array_element (`self.CurrentComponents`)
    (if (`SceneComponent.IsSimulatingPhysics` _array_element "None")
      (`PrimitiveComponent.AddImpulse` _array_element (* (+ (* (`self.CurrentDirection`) (`self.CurrentStrength`)) (`KismetMathLibrary.MakeVector` 0.0 0.0 (`self.Z_WaveSurge`))) 0.05) "None" false)
      (set `self.CurrentDirection` (`KismetMathLibrary.Normal` (`KismetMathLibrary.MakeVector` (`KismetMathLibrary.Sin` (* _returnvalue_2 0.3)) (`KismetMathLibrary.Cos` (* _returnvalue_2 0.4)) (+ (+ (* (`KismetMathLibrary.Sin` (* _returnvalue_2 0.2)) 0.15) 0.5) (`self.Z_WaveSurge`)))))
      (`KismetSystemLibrary.DrawDebugArrow` _returnvalue (+ _returnvalue (* (`self.CurrentDirection`) 500.0)) 50.0 (struct :`R` 1.0 :`B` 0.027822 :`A` 1.0))
      (set `self.Z_WaveSurge` (`KismetMathLibrary.FInterpTo` (`self.Z_WaveSurge`) 0.0 (stale `self.ReceiveTick` DeltaSeconds) 0.08))
      (if (and (< (`self.Z_WaveSurge`) 50.0) (`self.IsWaveActive`))
        (set `self.IsWaveActive` false)
        (`KismetSystemLibrary.PrintString` "Dalga bitti")))))

(event `self.ReceiveTick`
  (params (DeltaSeconds :type "Float (single-precision)"))
  (bind _currentstrength (`self.CurrentStrength`))
  (bind (_x _y) (`KismetMathLibrary.BreakVector2D` (`self.CausticsOffset`)))
  (set `self.CurrentStrength` (`KismetMathLibrary.FInterpTo` (`self.CurrentStrength`) (`self.TargetStrength`) DeltaSeconds 1.0))
  (`KismetMaterialLibrary.SetScalarParameterValue` "/Game/kelp/kelp/StaticMeshes/MPC_Radar.MPC_Radar" "CurrentIntensity" (`KismetMathLibrary.MapRangeClamped` _currentstrength 0.0 100.0 0.5 0.1))
  (`KismetMaterialLibrary.SetScalarParameterValue` "/Game/kelp/kelp/StaticMeshes/MPC_Radar.MPC_Radar" "CurrentSpeed" (`KismetMathLibrary.MapRangeClamped` _currentstrength 0.0 2.0 0.5 1.0))
  (set `self.CausticsVelocity` (+ (* (`self.CausticsVelocity`) DeltaSeconds) (make `LinearColor` _x _y)))
  (bind _output_get (set `self.CausticsOffset` (`KismetMathLibrary.Conv_VectorToVector2D` (+ (* (* (* (`self.CurrentStrength`) (`self.CurrentDirection`)) DeltaSeconds) 0.0003) (`self.CausticsOffset`)))))
  (bind (_x_2 _y_2) (`KismetMathLibrary.BreakVector2D` _output_get))
  (`KismetMaterialLibrary.SetVectorParameterValue` "/Game/kelp/kelp/StaticMeshes/MPC_Radar.MPC_Radar" "CurrentDirection" (make `LinearColor` _x_2 _y_2)))

(event `self.Box.OnComponentBeginOverlap`
  (params (OverlappedComponent :type "PrimitiveComponent Object Reference") (OtherActor :type "Actor Object Reference") (OtherComp :type "PrimitiveComponent Object Reference") (OtherBodyIndex :type Integer) (bFromSweep :type Boolean) (SweepResult :type "HitResult Structure (by ref)"))
  (if (`SceneComponent.IsSimulatingPhysics` OtherComp "None")
    (`KismetArrayLibrary.Array_AddUnique` (`self.CurrentComponents`) OtherComp)))

(event `self.Box.OnComponentEndOverlap`
  (params (OverlappedComponent :type "PrimitiveComponent Object Reference") (OtherActor :type "Actor Object Reference") (OtherComp :type "PrimitiveComponent Object Reference") (OtherBodyIndex :type Integer))
  (`KismetArrayLibrary.Array_RemoveItem` (`self.CurrentComponents`) OtherComp))

(fn `UserConstructionScript`)