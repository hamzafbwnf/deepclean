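; Trash spawner that feeds pooled BP_LightTrash actors into a box volume at random points.
; On BeginPlay it sets global distance field console variables, gathers the placed BP_LightTrash actors and deactivates them all.
; A fast looping timer activates one pooled piece per tick while under the active cap, treating actors far below the world as free.
; It updates active and remaining pool counters on each spawn.
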(event `self.ReceiveBeginPlay`
  (`KismetSystemLibrary.ExecuteConsoleCommand` "r.GlobalDistanceField.MaxCacheInvalDistance 2" null)
  (`KismetSystemLibrary.ExecuteConsoleCommand` "r.GlobalDistanceField.UpdateInterval 1" null)
  (bind _outactors (`GameplayStatics.GetAllActorsOfClass` "/Game/Trash/PointTrash/BP_LightTrash.BP_LightTrash_C"))
  (bind _output_get (set `self.trachpool` _outactors))
  (for _array_element _output_get
    (`/Game/Trash/PointTrash/BP_LightTrash.Deactivate` _array_element))
  (`KismetSystemLibrary.K2_SetTimer` null "SpawnSingleTrash" 0.1 true))

(event `SpawnSingleTrash`
  (bind (_origin _boxextent) (`KismetSystemLibrary.GetComponentBounds` (`self.Box`)))
  (if (< (`self.CurrentActiveTrash`) (`self.MaxActiveTrash`))
    (for _array_element (`self.trachpool`)
      (bind (_returnvalue_x _returnvalue_y _returnvalue_z) (`KismetMathLibrary.BreakVector` (`self.K2_GetActorLocation` _array_element)))
      (if (< _returnvalue_z -9000.0)
        (`/Game/Trash/PointTrash/BP_LightTrash.Activate` _array_element (`KismetMathLibrary.RandomPointInBoundingBox` _origin _boxextent))
        (set `self.CurrentActiveTrash` (+ (`self.CurrentActiveTrash`) 1))
        (set `self.TotalTrashPool` (- (`self.TotalTrashPool`) 1))
        (break)))))

(event `delayspawn`
  (`self.SpawnSingleTrash`))

(fn `UserConstructionScript`)