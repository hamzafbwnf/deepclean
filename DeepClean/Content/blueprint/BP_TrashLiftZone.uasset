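; BP_TrashLiftZone is a placeable volume that detects physics-simulating components tagged TrashLiftable and reports them to the level's BP_TrashLiftManager.
; Entering LiftArea tracks and registers a component; only leaving LiftReleaseArea unregisters it, giving hysteresis at the zone boundary.
; The construction script sizes and offsets both boxes from zone dimensions, lift height and surface inset, with extra side and top margins for release.
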(event `self.ReceiveBeginPlay`
  (bind _returnvalue (`GameplayStatics.GetActorOfClass` "/Game/blueprint/BP_TrashLiftManager.BP_TrashLiftManager_C"))
  (set `self.LiftManager` _returnvalue))

(event `self.LiftArea.OnComponentBeginOverlap`
  (params (OverlappedComponent :type "PrimitiveComponent Object Reference") (OtherActor :type "Actor Object Reference") (OtherComp :type "PrimitiveComponent Object Reference") (OtherBodyIndex :type Integer) (bFromSweep :type Boolean) (SweepResult :type "HitResult Structure (by ref)"))
  (bind _trackedcomponents (`self.TrackedComponents`))
  (bind _liftmanager (`self.LiftManager`))
  (if (and (`SceneComponent.IsSimulatingPhysics` OtherComp "None") (`ActorComponent.ComponentHasTag` OtherComp "TrashLiftable"))
    (if (not (`KismetArrayLibrary.Array_Contains` _trackedcomponents OtherComp))
      (`KismetArrayLibrary.Array_AddUnique` _trackedcomponents OtherComp)
      (`/Engine/EditorBlueprintResources/StandardMacros.IsValid` _liftmanager
        (:`Is Valid`
          (`/Game/blueprint/BP_TrashLiftManager.RegisterLiftComponent` _liftmanager OtherComp))))))

(event `self.LiftReleaseArea.OnComponentEndOverlap`
  (params (OverlappedComponent :type "PrimitiveComponent Object Reference") (OtherActor :type "Actor Object Reference") (OtherComp :type "PrimitiveComponent Object Reference") (OtherBodyIndex :type Integer))
  (bind _trackedcomponents (`self.TrackedComponents`))
  (bind _liftmanager (`self.LiftManager`))
  (if (`KismetArrayLibrary.Array_Contains` _trackedcomponents OtherComp)
    (`KismetArrayLibrary.Array_RemoveItem` _trackedcomponents OtherComp)
    (`/Engine/EditorBlueprintResources/StandardMacros.IsValid` _liftmanager
      (:`Is Valid`
        (`/Game/blueprint/BP_TrashLiftManager.UnregisterLiftComponent` _liftmanager OtherComp)))))

(event `self.LiftArea.OnComponentEndOverlap`
  (params (OverlappedComponent :type "PrimitiveComponent Object Reference") (OtherActor :type "Actor Object Reference") (OtherComp :type "PrimitiveComponent Object Reference") (OtherBodyIndex :type Integer)))

(fn `UserConstructionScript`
  (bind _liftarea (`self.LiftArea`))
  (bind _liftreleasearea (`self.LiftReleaseArea`))
  (bind _returnvalue (* (+ (`self.LiftHeight`) (`self.ReleaseTopMargin`)) 0.5))
  (`|ExecutionSequence`
    (:`then_0`
      (`BoxComponent.SetBoxExtent` _liftarea (`KismetMathLibrary.MakeVector` (* (`self.ZoneLength`) 0.5) (* (`self.ZoneWidth`) 0.5) (* (+ (`self.LiftHeight`) (`self.SurfaceInset`)) 0.5)) true)
      (`SceneComponent.K2_SetRelativeLocation` _liftarea (`KismetMathLibrary.MakeVector` 0.0 0.0 (* (- (`self.LiftHeight`) (`self.SurfaceInset`)) 0.5)) false false))
    (:`then_1`
      (`BoxComponent.SetBoxExtent` _liftreleasearea (`KismetMathLibrary.MakeVector` (+ (* (`self.ZoneLength`) 0.5) (`self.ReleaseSideMargin`)) (+ (* (`self.ZoneWidth`) 0.5) (`self.ReleaseSideMargin`)) _returnvalue) true)
      (`SceneComponent.K2_SetRelativeLocation` _liftreleasearea (`KismetMathLibrary.MakeVector` 0.0 0.0 (- _returnvalue (`self.SurfaceInset`))) false false))))