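; BP_LightTrash is a trash actor that can be switched off and reused at a new location, in the manner of a pooled object.
; Deactivate parks it far below the world and turns off collision, tick and the mesh's distance field lighting, while Activate moves it to a supplied location and restores them.
; BeginPlay nudges it slightly upward; radar, teleport and debug nodes are left unconnected.
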(event `self.ReceiveBeginPlay`
  (`self.K2_SetActorLocation` (+ (`self.K2_GetActorLocation`) (0.0 0.0 0.1)) false true)
  (`PrimitiveComponent.SetAffectDistanceFieldLighting` (`self.TrashMesh`) true))

(event `self.ReceiveTick`
  (params (DeltaSeconds :type "Float (single-precision)")))

(event `Deactivate`
  (bind (_returnvalue_x _returnvalue_y) (`KismetMathLibrary.BreakVector` (`self.K2_GetActorLocation`)))
  (`self.K2_SetActorLocation` (`KismetMathLibrary.MakeVector` _returnvalue_x _returnvalue_y -10000.0))
  (`self.SetActorEnableCollision` false)
  (`self.SetActorTickEnabled` false)
  (`PrimitiveComponent.SetAffectDistanceFieldLighting` (`self.TrashMesh`) false))

(event `Activate`
  (params (newlocation :type "Vector Structure"))
  (`self.K2_SetActorLocation` newlocation)
  (`self.SetActorEnableCollision` true)
  (`self.SetActorTickEnabled` true)
  (`PrimitiveComponent.SetAffectDistanceFieldLighting` (`self.TrashMesh`) true))

(event `self.TrashMesh.OnComponentSleep`
  (params (SleepingComponent :type "PrimitiveComponent Object Reference") (BoneName :type Name)))

(fn `UserConstructionScript`)