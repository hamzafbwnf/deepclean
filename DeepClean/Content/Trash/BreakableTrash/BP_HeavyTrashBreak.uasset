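; BP_HeavyTrashBreak is a breakable heavy trash actor that shatters into three BP_LightTrash pieces and destroys itself.
; It breaks on a hard enough impact from anything except the player character, or on a non-player overlap while TrashMesh is not simulating physics.
; Both triggers share one spawn path that scatters pieces in a flat box around the Hit event's location, which the overlap path does not set.
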(event `self.ReceiveHit`
  (params (MyComp :type "PrimitiveComponent Object Reference") (Other :type "Actor Object Reference") (OtherComp :type "PrimitiveComponent Object Reference") (bSelfMoved :type Boolean) (HitLocation :type "Vector Structure") (HitNormal :type "Vector Structure") (NormalImpulse :type "Vector Structure") (Hit :type "HitResult Structure (by ref)"))
  (if (and (> (`KismetMathLibrary.VSize` NormalImpulse) 1000.0) (!= Other (`GameplayStatics.GetPlayerCharacter` 0)))
    (for _ (range 1 4) :!label _label
      (`|SpawnActorFromClass` "/Game/Trash/PointTrash/BP_LightTrash.BP_LightTrash_C" (`KismetMathLibrary.Conv_VectorToTransform` (`KismetMathLibrary.RandomPointInBoundingBox` HitLocation (12.0 15.0 0.0))) "Undefined" "MultiplyWithRoot" null null))
    (`self.K2_DestroyActor`)))

(event `self.ReceiveActorBeginOverlap`
  (params (OtherActor :type "Actor Object Reference"))
  (if (and (!= OtherActor (`GameplayStatics.GetPlayerCharacter` 0)) (not (`SceneComponent.IsSimulatingPhysics` (`self.TrashMesh`) "None")))
    (goto _label)))

(fn `UserConstructionScript`)